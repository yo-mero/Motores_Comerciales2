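; Traffic light actor that cycles endlessly through red, yellow and green from BeginPlay.
; The Luces event lights one lamp at a time by swapping materials on the Rojo, Amarillo and Verde components, setting the other two to glass.
; Delays hold red and yellow briefly and green for longer, then Luces calls itself to repeat the loop.
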(event `self.ReceiveBeginPlay`
  (`self.Luces`))

(event `Luces`
  (`PrimitiveComponent.SetMaterial` (`self.Rojo`) 0 "/Game/Assets/textures/Red_Stop.Red_Stop")
  (`PrimitiveComponent.SetMaterial` (`self.Amarillo`) 0 "/Game/MAterials/Glass_mat_Inst.Glass_mat_Inst")
  (`PrimitiveComponent.SetMaterial` (`self.Verde`) 0 "/Game/MAterials/Glass_mat_Inst.Glass_mat_Inst")
  (`KismetSystemLibrary.Delay` 2.0)
  (`PrimitiveComponent.SetMaterial` (`self.Rojo`) 0 "/Game/MAterials/Glass_mat_Inst.Glass_mat_Inst")
  (`PrimitiveComponent.SetMaterial` (`self.Amarillo`) 0 "/Game/Assets/textures/Yellow_light.Yellow_light")
  (`PrimitiveComponent.SetMaterial` (`self.Verde`) 0 "/Game/MAterials/Glass_mat_Inst.Glass_mat_Inst")
  (`KismetSystemLibrary.Delay` 2.0)
  (`PrimitiveComponent.SetMaterial` (`self.Rojo`) 0 "/Game/MAterials/Glass_mat_Inst.Glass_mat_Inst")
  (`PrimitiveComponent.SetMaterial` (`self.Amarillo`) 0 "/Game/MAterials/Glass_mat_Inst.Glass_mat_Inst")
  (`PrimitiveComponent.SetMaterial` (`self.Verde`) 0 "/Game/Assets/textures/Green_light.Green_light")
  (`KismetSystemLibrary.Delay` 10.0)
  (`self.Luces`))

(fn `UserConstructionScript`)