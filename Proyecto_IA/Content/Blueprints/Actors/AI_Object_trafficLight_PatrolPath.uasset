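; Traffic light actor that endlessly alternates between red and green, with a purely visual cycle.
; BeginPlay starts ChangeLight, which swaps materials on the RedLight and GreenLight components so one is lit while the other shows glass.
; A fixed delay holds each state before the event calls itself again, forming a latent loop without Tick or timers.
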(event `self.ReceiveBeginPlay`
  (`self.ChangeLight`))

(event `ChangeLight`
  (`PrimitiveComponent.SetMaterial` (`self.RedLight`) 0 "/Game/Assets/textures/Red_Stop.Red_Stop")
  (`PrimitiveComponent.SetMaterial` (`self.GreenLight`) 0 "/Game/MAterials/Glass_mat_Inst.Glass_mat_Inst")
  (`KismetSystemLibrary.Delay` 10.0)
  (`PrimitiveComponent.SetMaterial` (`self.RedLight`) 0 "/Game/MAterials/Glass_mat.Glass_mat")
  (`PrimitiveComponent.SetMaterial` (`self.GreenLight`) 0 "/Game/Assets/textures/Green_light.Green_light")
  (`KismetSystemLibrary.Delay` 10.0)
  (`self.ChangeLight`))

(fn `UserConstructionScript`
  (`parent.UserConstructionScript`))